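; Flame pillar actor that makes its flame light flicker continuously.
; On BeginPlay it randomly picks one of two intensity timelines to start, and each starts the other when finished, so they alternate in a loop.
; Each timeline update feeds its curve value to ScaleFlameIntensity, which multiplies it by BaseIntensity and sets the light's intensity.
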(event Custom|StartTImeline_1
  (bind _flameintensity1 (Timeline|FlameIntensityTimeline PlayFromStart)
    (:Update
      (CallFunction|ScaleFlameIntensity _flameintensity1))
    (:Finished
      (CallFunction|StartTimeline2))))

(event Custom|StartTimeline_2
  (bind _flameintensity2 (Timeline|FlameIntensity_2 PlayFromStart)
    (:Update
      (CallFunction|ScaleFlameIntensity _flameintensity2))
    (:Finished
      (CallFunction|StartTImeline1))))

(event Custom|ChooseTimeline
  (switch int (Math|Random|RandomIntegerinRange 0 1)
    (:Default
      (CallFunction|StartTimeline2 :!label _label))
    (:0
      (CallFunction|StartTImeline1))
    (:1
      (goto _label))))

(event EventBeginPlay
  (CallFunction|ChooseTimeline))

(event Collision|EventActorBeginOverlap
  (params (OtherActor :type Actor%20Object%20Reference)))

(event EventTick
  (params (DeltaSeconds :type Float%20%28single-precision%29)))

(fn ConstructionScript)

(fn ScaleFlameIntensity
  (params (Intensity :type Float%20%28double-precision%29))
  (Rendering|Components|Light|SetIntensity (Variables|Default|GetFlameLight) (* Intensity (Variables|Default|GetBaseIntensity))))